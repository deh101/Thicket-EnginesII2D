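; BP_Elder is a story NPC that delivers a short cryptic speech when the BP_Thicket player pawn first overlaps it.
; A DoOnce gate flags ElderSpeaking and steps the text render through timed lines using Delays, starting from ElderText's default value.
; Afterwards it hides the speech, plays the non-looping Elder_leaves flipbook and reveals a second text, TextRenderJump, which is hidden on end overlap.
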(event EventBeginPlay)

(event Collision|EventActorBeginOverlap
  (params (OtherActor :type Actor%20Object%20Reference))
  (Utilities|Casting|CastToBP_Thicket (Game|Player|GetPlayerPawn 0))
  (Utilities|FlowControl|DoOnce false
    (:Completed
      (Rendering|SetVisibility (Variables|Default|GetTextRender) true false)
      (Variables|Default|SetElderSpeaking true)
      (Rendering|Components|TextRender|SetText (Variables|Default|GetTextRender) (Variables|Default|GetElderText))
      (Variables|Default|SetElderText "As it always was.")
      (Utilities|FlowControl|Delay 2.0)
      (Rendering|Components|TextRender|SetText (Variables|Default|GetTextRender) (Variables|Default|GetElderText))
      (Variables|Default|SetElderText "You must succeed...")
      (Utilities|FlowControl|Delay 2.0)
      (Rendering|Components|TextRender|SetText (Variables|Default|GetTextRender) (Variables|Default|GetElderText))
      (Variables|Default|SetElderText "where those who came before failed.")
      (Utilities|FlowControl|Delay 2.0)
      (Rendering|Components|TextRender|SetText (Variables|Default|GetTextRender) (Variables|Default|GetElderText))
      (Variables|Default|SetElderText "Find the tree...")
      (Utilities|FlowControl|Delay 2.0)
      (Rendering|Components|TextRender|SetText (Variables|Default|GetTextRender) (Variables|Default|GetElderText))
      (Variables|Default|SetElderText "Break the cycle!")
      (Utilities|FlowControl|Delay 2.0)
      (Rendering|Components|TextRender|SetText (Variables|Default|GetTextRender) (Variables|Default|GetElderText))
      (Utilities|FlowControl|Delay 2.0)
      (Rendering|SetVisibility (Variables|Default|GetTextRender) false false)
      (Sprite|SetFlipbook (Variables|Default|GetElderFlipbook) "/Game/SpriteAssets/Interactables/Elder/elder_leaves.elder_leaves")
      (Components|Timeline|PlayfromStart (Variables|Default|GetElderFlipbook))
      (Rendering|SetVisibility (Variables|Default|GetTextRenderJump) true false))))

(event EventTick
  (params (DeltaSeconds :type Float%20%28single-precision%29)))

(event Collision|EventActorEndOverlap
  (params (OtherActor :type Actor%20Object%20Reference))
  (Utilities|Casting|CastToBP_Thicket (Game|Player|GetPlayerPawn 0))
  (Rendering|SetVisibility (Variables|Default|GetTextRenderJump) false false))

(fn ConstructionScript
  (Components|Timeline|SetLooping (Variables|Default|GetElderFlipbook) false))