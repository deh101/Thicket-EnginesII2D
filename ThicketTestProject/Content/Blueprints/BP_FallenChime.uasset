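; BP_FallenChime is an overlap-triggered ending sequence that finishes by quitting the game.
; On overlap it casts the player pawn to BP_Thicket, hides its flipbook, disables input and moves it to a fixed Z.
; A chain of delays plays its own non-looping flipbook, hides the sprite, switches to holding and look-up animations, then reveals a black tilemap background and text before quitting.
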(event EventBeginPlay)

(event Collision|EventActorBeginOverlap
  (params (OtherActor :type Actor%20Object%20Reference))
  (bind _asbp_thicket (Utilities|Casting|CastToBP_Thicket (Game|Player|GetPlayerPawn 0)))
  (Rendering|SetVisibility (Variables|/Game/Blueprints/BP_Thicket.BP_Thicket_C|GetThicketPaperFlipbook _asbp_thicket) false false)
  (Input|DisableInput _asbp_thicket 0)
  (Transformation|SetActorLocation _asbp_thicket (Math|Vector|MakeVector (.x (Transformation|GetActorLocation _asbp_thicket)) (.y (Transformation|GetActorLocation _asbp_thicket)) -2536.0) false false)
  (Rendering|SetVisibility (Variables|Default|GetPaperFlipbook) true false)
  (Components|Timeline|PlayfromStart (Variables|Default|GetPaperFlipbook))
  (Utilities|FlowControl|Delay 1.0)
  (Rendering|SetVisibility (Variables|Default|GetPaperSprite) false false)
  (Sprite|SetFlipbook (Variables|Default|GetPaperFlipbook) "/Game/SpriteAssets/Player/ChimePickup/holding.holding")
  (Utilities|FlowControl|Delay 3.0)
  (Sprite|SetFlipbook (Variables|Default|GetPaperFlipbook) "/Game/SpriteAssets/Player/ChimePickup/LookupHolding.LookupHolding")
  (Utilities|FlowControl|Delay 0.5)
  (Rendering|SetVisibility (Variables|Default|GetBLACK_BG_TILEMAP) true false)
  (Utilities|FlowControl|Delay 3.0)
  (Rendering|SetVisibility (Variables|Default|GetTextRender) true false)
  (Utilities|FlowControl|Delay 6.0)
  (Game|QuitGame 0 "Quit" false))

(event EventTick
  (params (DeltaSeconds :type Float%20%28single-precision%29)))

(fn ConstructionScript
  (Components|Timeline|SetLooping (Variables|Default|GetPaperFlipbook) false))