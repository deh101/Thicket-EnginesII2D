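; BP_Mushroom2 is a Paper2D mushroom that plays a boing animation and sound when overlapped.
; On any actor overlap, it checks only that player pawn 0 is a BP_Thicket, not which actor overlapped.
; It then restarts its non-looping flipbook and plays one of four random boing cues at its location.
; The construction script pins its X position and rotation to fixed values, keeping Y and Z as placed.
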(event Collision|EventActorBeginOverlap
  (params (OtherActor :type Actor%20Object%20Reference))
  (Utilities|Casting|CastToBP_Thicket (Game|Player|GetPlayerPawn 0))
  (Components|Timeline|PlayfromStart (Variables|Default|GetPaperFlipbook))
  (Audio|PlaySoundatLocation (Utilities|Select :Index (Math|Random|RandomIntegerinRange 0 3) :Option%200 "/Game/SpriteAssets/Sounds/Boing/boing_sounds1_Cue.boing_sounds1_Cue" :Option%201 "/Game/SpriteAssets/Sounds/Boing/boing_sounds2_Cue.boing_sounds2_Cue" :Option%202 "/Game/SpriteAssets/Sounds/Boing/boing_sounds3_Cue.boing_sounds3_Cue" :Option%203 "/Game/SpriteAssets/Sounds/Boing/boing_sounds4_Cue.boing_sounds4_Cue") (Transformation|GetActorLocation) "0, 0, 0" 1.0 1.0 0.0 0 0 0))

(fn ConstructionScript
  (bind _returnvalue (Transformation|GetActorLocation))
  (Components|Timeline|SetLooping (Variables|Default|GetPaperFlipbook) false)
  (Transformation|SetActorLocation (Math|Vector|MakeVector 0.2 (.y _returnvalue) (.z _returnvalue)) false false)
  (Transformation|SetActorRotation "0,90.000000, 0"))