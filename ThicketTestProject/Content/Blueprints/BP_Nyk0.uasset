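; BP_Nyk0 is a Paper2D character that tells the player they have found an unfinished secret section and teases a sequel.
; On any actor overlap, if the player pawn is BP_Thicket, it shows a popup sprite and text render, stepping through lines and sprite swaps with chained Delays.
; It then hides popup, text and flipbook and plays a boing sound.
; The overlapping actor is never checked, and nothing disables replay.
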(event EventBeginPlay)

(event Collision|EventActorBeginOverlap
  (params (OtherActor :type Actor%20Object%20Reference))
  (Utilities|Casting|CastToBP_Thicket (Game|Player|GetPlayerPawn 0))
  (Rendering|SetVisibility (Variables|Default|GetPopupSprite) true false)
  (Rendering|SetVisibility (Variables|Default|GetTextRender) true false)
  (Rendering|Components|TextRender|SetText (Variables|Default|GetTextRender) (Variables|Default|GetNYK0Text))
  (Utilities|FlowControl|Delay 2.0)
  (Variables|Default|SetNYK0Text "You aren't Supposed to be here!")
  (Rendering|Components|TextRender|SetText (Variables|Default|GetTextRender) (Variables|Default|GetNYK0Text))
  (Rendering|Components|Sprite|SetSprite (Variables|Default|GetPopupSprite) "/Game/SpriteAssets/Interactables/NYK0/Sprites/Popups/NYK0_popup4_Sprite.NYK0_popup4_Sprite")
  (Utilities|FlowControl|Delay 2.0)
  (Variables|Default|SetNYK0Text "This section is a secret!")
  (Rendering|Components|TextRender|SetText (Variables|Default|GetTextRender) (Variables|Default|GetNYK0Text))
  (Rendering|Components|Sprite|SetSprite (Variables|Default|GetPopupSprite) "/Game/SpriteAssets/Interactables/NYK0/Sprites/Popups/NYK0_popup1_Sprite.NYK0_popup1_Sprite")
  (Utilities|FlowControl|Delay 2.0)
  (Variables|Default|SetNYK0Text "And it's still in developpment!")
  (Rendering|Components|TextRender|SetText (Variables|Default|GetTextRender) (Variables|Default|GetNYK0Text))
  (Utilities|FlowControl|Delay 2.0)
  (Variables|Default|SetNYK0Text "You'll find the rest in the sequel ;)")
  (Rendering|Components|TextRender|SetText (Variables|Default|GetTextRender) (Variables|Default|GetNYK0Text))
  (Rendering|Components|Sprite|SetSprite (Variables|Default|GetPopupSprite) "/Game/SpriteAssets/Interactables/NYK0/Sprites/Popups/NYK0_popup6_Sprite.NYK0_popup6_Sprite")
  (Utilities|FlowControl|Delay 4.0)
  (Rendering|SetVisibility (Variables|Default|GetPopupSprite) false false)
  (Rendering|SetVisibility (Variables|Default|GetNYK0Flipbook) false false)
  (Rendering|SetVisibility (Variables|Default|GetTextRender) false false)
  (Audio|PlaySoundatLocation "/Game/SpriteAssets/Sounds/Boing/boing_sounds1_Cue.boing_sounds1_Cue" (Transformation|GetActorLocation) "0, 0, 0" 1.0 1.0 0.0 0 0 0))

(event EventTick
  (params (DeltaSeconds :type Float%20%28single-precision%29)))

(fn ConstructionScript)