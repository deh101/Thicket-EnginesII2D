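; Thicket is a Paper2D side-view playable character with hand-written movement on the Y/Z plane: walk, variable-height jump and one dash per landing.
; A movement-mode state selects gravity, speed limits and flipbook.
; Each tick, input, gravity, jump and dash accumulate velocity, resolved by a swept move that slides along surfaces and derives actual velocity.
; Upward-facing hits set Grounded and restart a tiny timer that triggers falling when contact stops.
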(event OnComponentHit(Box)
  (params (HitComponent :type Primitive%20Component%20Object%20Reference) (OtherActor :type Actor%20Object%20Reference) (OtherComp :type Primitive%20Component%20Object%20Reference) (NormalImpulse :type Vector :default "0, 0, 0") (Hit :type Hit%20Result%20Structure%20%28by%20ref%29))
  (if (>= (Math|Vector|DotProduct (.normal Hit) "0, 0,1.000000") 0.01)
    (CallFunction|Grounded)))

(event EventBeginPlay)

(event EventTick
  (params (DeltaSeconds :type Float%20%28single-precision%29))
  (Utilities|FlowControl|Sequence
    (:then_0
      (Gravity|Gravity)
      (Jump|Jumping)
      (Dash|Dashing))
    (:then_1
      (CallFunction|Animations))
    (:then_2
      (Movement|ResolveMovement))))

(event Input|ActionEvents|InputActionJump
  (params (Key :type Key%20Structure))
  (:Pressed
    (Jump|StartJump))
  (:Released
    (Jump|StopJump true)))

(event Input|ActionEvents|InputActionDash
  (params (Key :type Key%20Structure))
  (:Pressed
    (Dash|StartDash)))

(event Input|AxisEvents|InputAxisMoveRight
  (params (AxisValue :type Float%20%28single-precision%29))
  (if (Utilities|Enum|NotEqual(Enum) (Variables|Movement|GetMovementMode) "NewEnumerator4")
    (Movement|AddVelocity "0,1.000000, 0" (* (Math|Float|Sign(Float) AxisValue) (Variables|Movement|GetMoveRightAccel)))))

(fn ConstructionScript
  (bind _returnvalue (Transformation|GetActorLocation))
  (Transformation|SetActorLocation (Math|Vector|MakeVector 0.0 (.y _returnvalue) (.z _returnvalue)) false false)
  (Variables|Default|SetSpawnPoint (Math|Vector|MakeVector (.x _returnvalue) (.y _returnvalue) (.z _returnvalue))))

(fn Gravity
  (bind _gravityacceleration (Variables|Gravity|GetGravityAcceleration))
  (Movement|AddVelocity "0, 0,-1.000000" (Utilities|Select :Index (Variables|Movement|GetMovementMode) :NewEnumerator0 _gravityacceleration :NewEnumerator1 0.0 :NewEnumerator3 (Variables|Gravity|GetRisingGravityAcceleration) :NewEnumerator2 _gravityacceleration :NewEnumerator4 0.0)))

(fn AddVelocity
  (params (Direction :type Vector) (Scale :type Float%20%28single-precision%29))
  (Variables|Movement|SetAddedVelocity (+ (* Direction (* Scale (Utilities|Time|GetWorldDeltaSeconds))) (Variables|Movement|GetAddedVelocity))))

(fn ResolveMovement
  (bind _movementmode (Variables|Movement|GetMovementMode))
  (bind _dashmaxspeed (Variables|Dash|GetDashMaxSpeed))
  (bind _maxwalkspeed (Variables|Movement|GetMaxWalkSpeed))
  (bind _jumpspeedcap (Variables|Jump|GetJumpSpeedCap))
  (bind _maxfallspeed (Variables|Gravity|GetMaxFallSpeed))
  (bind _movementmode_2 (Variables|Movement|GetMovementMode))
  (bind _returnvalue (Utilities|Select :Index _movementmode :NewEnumerator0 _maxwalkspeed :NewEnumerator1 _maxwalkspeed :NewEnumerator3 _maxwalkspeed :NewEnumerator2 _maxwalkspeed :NewEnumerator4 _dashmaxspeed))
  (LocalVariables|SetLocationBefore (Transformation|GetActorLocation))
  (Utilities|FlowControl|Sequence
    (:then_0
      (bind _sweephitresult (Transformation|SetActorLocation (+ (Transformation|GetActorLocation) (* (Math|Vector|MakeVector 0.0 (Math|Float|Clamp(Float) (|InstantAccel (.Y (Math|Vector|BreakVector (+ (Variables|Movement|GetVelocity) (Variables|Movement|GetAddedVelocity))))) (* _returnvalue -1.0) _returnvalue) (Math|Float|Clamp(Float) (.Z (Math|Vector|BreakVector (+ (Variables|Movement|GetVelocity) (Variables|Movement|GetAddedVelocity)))) (Utilities|Select :Index (Variables|Movement|GetMovementMode) :NewEnumerator0 _maxfallspeed :NewEnumerator1 _maxfallspeed :NewEnumerator3 _maxfallspeed :NewEnumerator2 _maxfallspeed :NewEnumerator4 0.0) (Utilities|Select :Index (Variables|Movement|GetMovementMode) :NewEnumerator0 0.0 :NewEnumerator1 _jumpspeedcap :NewEnumerator3 _jumpspeedcap :NewEnumerator2 _jumpspeedcap :NewEnumerator4 0.0))) (Utilities|Time|GetWorldDeltaSeconds))) true false))
      (bind _output_get (LocalVariables|SetLocalSweep _sweephitresult))
      (while (and (.bBlockingHit (Collision|BreakHitResult _output_get)) (> (Math|Vector|VectorLength (- (- (.TraceEnd (Collision|BreakHitResult _output_get)) (.TraceStart (Collision|BreakHitResult _output_get))) (* (.ImpactNormal (Collision|BreakHitResult _output_get)) (Math|Vector|DotProduct (.ImpactNormal (Collision|BreakHitResult _output_get)) (- (.TraceEnd (Collision|BreakHitResult _output_get)) (.TraceStart (Collision|BreakHitResult _output_get))))))) 0.0))
        (bind _sweephitresult_2 (Transformation|SetActorLocation (+ (Transformation|GetActorLocation) (+ (* (.ImpactNormal (Collision|BreakHitResult _output_get)) 0.0125) (- (- (.TraceEnd (Collision|BreakHitResult _output_get)) (.TraceStart (Collision|BreakHitResult _output_get))) (* (.ImpactNormal (Collision|BreakHitResult _output_get)) (Math|Vector|DotProduct (.ImpactNormal (Collision|BreakHitResult _output_get)) (- (.TraceEnd (Collision|BreakHitResult _output_get)) (.TraceStart (Collision|BreakHitResult _output_get)))))))) true false))
        (LocalVariables|SetLocalSweep _sweephitresult_2)))
    (:then_1
      (Utilities|FlowControl|Sequence
        (:then_0
          (Variables|Movement|SetVelocity (/ (- (Transformation|GetActorLocation) (LocalVariables|GetLocationBefore)) (Utilities|Time|GetWorldDeltaSeconds)))
          (Variables|Movement|SetAddedVelocity "0, 0, 0"))
        (:then_1
          (if (or (Utilities|Enum|Equal(Enum) _movementmode_2 "NewEnumerator1") (Utilities|Enum|Equal(Enum) _movementmode_2 "NewEnumerator3"))
            (if (<= (.z (Variables|Movement|GetVelocity)) 0.0)
              (Movement|ChangeMovement "NewEnumerator2"))))))))

(fn ChangeMovement
  (params (NewMovement :type EMovement%20Enum :default "NewEnumerator0"))
  (LocalVariables|SetOldMovement (Variables|Movement|GetMovementMode))
  (switch Utilities|FlowControl|Switch|SwitchonEMovement NewMovement
    (:NewEnumerator0
      (if (Utilities|Enum|NotEqual(Enum) (Variables|Movement|GetMovementMode) "NewEnumerator4") :!label _label
        (Variables|Movement|SetMovementMode NewMovement :!label _label_2)
        (return (Utilities|Enum|NotEqual(Enum) (LocalVariables|GetOldMovement) NewMovement))))
    (:NewEnumerator1
      (goto _label))
    (:NewEnumerator3
      (goto _label))
    (:NewEnumerator2
      (if (Utilities|Enum|NotEqual(Enum) (Variables|Movement|GetMovementMode) "NewEnumerator1")
        (goto _label_2)))
    (:NewEnumerator4
      (goto _label_2))))

(fn Ungrounded
  (if (not (CallFunction|InAir))
    (Movement|ChangeMovement "NewEnumerator2")))

(fn InAir
  (bind _movementmode (Variables|Movement|GetMovementMode))
  (return (Math|Boolean|ORBoolean (Utilities|Enum|Equal(Enum) _movementmode "NewEnumerator1") (Utilities|Enum|Equal(Enum) _movementmode "NewEnumerator2") (Utilities|Enum|Equal(Enum) _movementmode "NewEnumerator3"))))

(fn StartJump
  (if (Utilities|Enum|Equal(Enum) (Variables|Movement|GetMovementMode) "NewEnumerator0")
    (Variables|Jump|SetJumpTimer 0.0)
    (Movement|ChangeMovement "NewEnumerator1")))

(fn Jumping
  (if (Utilities|Enum|Equal(Enum) (Variables|Movement|GetMovementMode) "NewEnumerator1")
    (Movement|AddVelocity "0, 0,1.000000" (Variables|Jump|GetJumpAcceleration))
    (bind _output_get (Variables|Jump|SetJumpTimer (+ (Variables|Jump|GetJumpTimer) (Utilities|Time|GetWorldDeltaSeconds))))
    (if (>= _output_get (Variables|Jump|GetJumpMaxDuration))
      (Jump|StopJump false))))

(fn StopJump
  (params (bSharp :type Boolean))
  (if (Utilities|Enum|Equal(Enum) (Variables|Movement|GetMovementMode) "NewEnumerator1")
    (Movement|ChangeMovement "NewEnumerator3")
    (if bSharp
      (Movement|AddVelocity "0, 0,-1.000000" (Math|Float|Absolute(Float) (/ (/ (.z (Variables|Movement|GetVelocity)) (Utilities|Time|GetWorldDeltaSeconds)) 1.5))))))

(fn Animations
  (Utilities|FlowControl|Sequence
    (:then_0
      (if (Utilities|Enum|NotEqual(Enum) (Variables|Movement|GetMovementMode) "NewEnumerator4")
        (Math|Float|CompareFloat (Math|Float|Sign(Float) (Input|AxisValues|GetMoveRight)) 0.0
          (:>
            (CallFunction|Look true))
          (:<
            (CallFunction|Look false)))))
    (:then_1
      (Sprite|SetFlipbook (Variables|Default|GetPaperFlipbook) (Utilities|Select :Index (Variables|Movement|GetMovementMode) :NewEnumerator0 (Utilities|Select :Index (Math|Float|Truncate (Math|Float|Absolute(Float) (Math|Float|Sign(Float) (.y (Variables|Movement|GetAddedVelocity))))) :Option%200 "/Game/SpriteAssets/Player/Idle/thicket_idle.thicket_idle" :Option%201 "/Game/SpriteAssets/Player/Walk/thicket_walk.thicket_walk") :NewEnumerator1 "/Game/SpriteAssets/Player/Jump/thicket_jump_full.thicket_jump_full" :NewEnumerator3 "/Game/SpriteAssets/Player/Jump/thicket_jump_full.thicket_jump_full" :NewEnumerator2 "/Game/SpriteAssets/Player/Jump/Flipbooks/thicket_jump_falling2.thicket_jump_falling2" :NewEnumerator4 "/Game/SpriteAssets/Player/Dash/thicket_dash_Flipbook.thicket_dash_Flipbook")))))

(fn StartDash
  (if (< (Variables|Dash|GetDashCounter) 1)
    (Utilities|FlowControl|Sequence
      (:then_0
        (Variables|Dash|SetDashCounter 1)
        (Variables|Dash|SetDashDirection (Variables|Default|GetLookDirection)))
      (:then_1
        (Variables|Dash|SetDashTimer 0.0)
        (Movement|ChangeMovement "NewEnumerator4")
        (Utilities|Time|ClearTimerbyFunctionName self "Ungrounded")))))

(fn Dashing
  (if (Utilities|Enum|Equal(Enum) (Variables|Movement|GetMovementMode) "NewEnumerator4")
    (Movement|AddVelocity (Variables|Dash|GetDashDirection) (Variables|Dash|GetDashAcceleration))
    (Variables|Dash|SetDashTimer (+ (Variables|Dash|GetDashTimer) (Utilities|Time|GetWorldDeltaSeconds)))
    (if (> (Variables|Dash|GetDashTimer) (Variables|Dash|GetDashDuration))
      (Dash|StopDash))))

(fn StopDash
  (Variables|Movement|SetMovementMode "NewEnumerator2"))

(fn Look
  (params (bLeft :type Boolean))
  (Transformation|SetRelativeRotation (Variables|Default|GetPaperFlipbook) (Math|Rotator|SelectRotator "0,90.000000, 0" "0.000000,270.000000,0.000000" bLeft) false false)
  (Variables|Default|SetLookDirection (select bLeft "0,1.000000, 0" "0,-1.000000, 0")))

(fn Grounded
  (Variables|Default|SetHeight (.z (Transformation|GetActorLocation)))
  (Movement|ChangeMovement "NewEnumerator0")
  (Variables|Dash|SetDashCounter 0)
  (Utilities|Time|SetTimerbyFunctionName self "Ungrounded" 1e-05))