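; BP_mushroom is an interactable mushroom with a Paper2D flipbook that makes the player jump, acting like a bounce pad.
; Its Interact function calls StartJump on the passed player reference and replays the flipbook animation from the start.
; The construction script sets flipbook looping from the AutoPlay variable, and the event graph holds only disabled default events.
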(event EventBeginPlay
  (|CallParentFunction) ; This node is disabled and will not be called.\nDrag off pins to build functionality.
)

(event Collision|EventActorBeginOverlap
  (params (OtherActor :type Actor%20Object%20Reference))
  (|CallParentFunction OtherActor) ; This node is disabled and will not be called.\nDrag off pins to build functionality.
)

(event EventTick
  (params (DeltaSeconds :type Float%20%28single-precision%29))
  (|CallParentFunction DeltaSeconds) ; This node is disabled and will not be called.\nDrag off pins to build functionality.
)

(fn ConstructionScript
  (Components|Timeline|SetLooping (Variables|Default|GetPaperFlipbook) (Variables|Default|GetAutoPlay)))

(fn Interact
  (params (PlayerRef :type BP%20Thicket%20Object%20Reference))
  (Default|StartJump PlayerRef)
  (Components|Timeline|PlayfromStart (Variables|Default|GetPaperFlipbook)))